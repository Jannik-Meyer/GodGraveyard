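; BP_Checkpoint is a checkpoint actor that updates the player's respawn location.
; On BeginPlay it caches every BP_Checkpoint in the level.
; When BP_Player overlaps its capsule, it writes the RespawnPoint world transform to SpawnTransform on BP_Gamemode_Base.
; It then deactivates the Niagara effect on all cached checkpoints and activates its own, so the effect marks the last touched checkpoint.
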(event `self.ReceiveBeginPlay`
  (bind _outactors (`GameplayStatics.GetAllActorsOfClass` "BP_Checkpoint_C"))
  (set `self.All checkpoints` _outactors))

(event `self.Capsule.OnComponentBeginOverlap`
  (params (OverlappedComponent :type "PrimitiveComponent Object Reference") (OtherActor :type "Actor Object Reference") (OtherComp :type "PrimitiveComponent Object Reference") (OtherBodyIndex :type Integer) (bFromSweep :type Boolean) (SweepResult :type "HitResult Structure (by ref)"))
  (cast `/Game/MyStuff/Blueprints/BP_Player` OtherActor)
  (bind _asbp_gamemode_base (cast `/Game/MyStuff/Blueprints/BP_Gamemode_Base` (`GameplayStatics.GetGameMode`)))
  (set `/Game/MyStuff/Blueprints/BP_Gamemode_Base.Spawn Transform` (`SceneComponent.K2_GetComponentToWorld` (`self.Respawn point`)) _asbp_gamemode_base)
  (for _array_element (`self.All checkpoints`)
    (`ActorComponent.SetActive` (`/Game/MyStuff/Blueprints/BP_Checkpoint.Niagara` _array_element) false false))
  (`ActorComponent.SetActive` (`self.Niagara`) true false))

(fn `UserConstructionScript`)