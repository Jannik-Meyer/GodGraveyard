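; Base game mode that manages UI, player respawning, pausing and ambient audio, with a GI_Puzzle game instance applying brightness.
; On BeginPlay it builds WBP_GameUI with gameplay and monologue layers, starts a desert ambience loop and caches the PlayerStart transform.
; Death fades the camera out, then spawns and possesses a new BP_Player at that transform.
; PauseGame toggles the pause stack, input mode and ambience; OpenSpeech forwards dialogue rows to the monologue widget.
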(event `self.ReceiveBeginPlay`
  (`self.SetUpGameInstance`)
  (`self.setUpUI`)
  (`self.SetupSpawn Transform`)
  (bind _returnvalue (`GameplayStatics.SpawnSound2D` "/Game/MyStuff/Sounds/Noise/atmo-desert-desert-loop-day-01.atmo-desert-desert-loop-day-01" 1.0 1.0 0.0 null))
  (set `self.Sounds` _returnvalue)
  (`self.Apply Brightness`))

(event `SetUpGameInstance`
  (bind _asgi_puzzle (cast `/Game/MyStuff/Blueprints/GI_Puzzle` (`GameplayStatics.GetGameInstance`)))
  (set `self.GAMe Instance` _asgi_puzzle))

(event `SetupSpawn Transform`
  (bind _returnvalue (`GameplayStatics.GetActorOfClass` "/Script/Engine.PlayerStart"))
  (set `self.Spawn Transform` (`self.GetTransform` _returnvalue)))

(event `PlayerDied`
  (`Widget.SetVisibility` (`self.GameUI`) "Hidden")
  (`PlayerCameraManager.StartCameraFade` :`self` (`GameplayStatics.GetPlayerCameraManager` 0) :`ToAlpha` 1.0 :`Duration` 1.0 :`bHoldWhenFinished` true)
  (`KismetSystemLibrary.Delay` 2.0)
  (`self.Player Spawn`))

(event `Player Spawn`
  (bind _spawn_transform (`self.Spawn Transform`))
  (bind _returnvalue (`|SpawnActorFromClass` "/Game/MyStuff/Blueprints/BP_Player.BP_Player_C" (`KismetMathLibrary.MakeTransform` (.location _spawn_transform) (`KismetMathLibrary.MakeRotator` 0.0 0.0 (.yaw (.rotation _spawn_transform)))) "Undefined" "MultiplyWithRoot" null null))
  (`Controller.Possess` (`GameplayStatics.GetPlayerController` 0) _returnvalue)
  (`KismetSystemLibrary.Delay` 1.0)
  (`PlayerCameraManager.StartCameraFade` :`self` (`GameplayStatics.GetPlayerCameraManager` 0) :`FromAlpha` 1.0 :`Duration` 1.0 :`bHoldWhenFinished` true)
  (`Widget.SetVisibility` (`self.GameUI`) "Visible"))

(event `PauseGame`
  (bind _returnvalue (`GameplayStatics.GetPlayerController` 0))
  (bind _pausestack (`/Game/MyStuff/UI/WBP_GameUI.PauseStack` (`self.GameUI`)))
  ;[1 1 1] pause game
  (if (not (`GameplayStatics.IsGamePaused`))
    (`CommonActivatableWidgetContainerBase.BP_AddWidget` _pausestack "/Game/MyStuff/UI/WBP_PauseMenuBase.WBP_PauseMenuBase_C")
    (`WidgetBlueprintLibrary.SetInputMode_UIOnlyEx` _returnvalue null)
    (set `PlayerController.bShowMouseCursor` true _returnvalue)
    (`GameplayStatics.SetGamePaused` true)
    (`AudioComponent.SetPaused` (`self.Sounds`) true)
    (else
      (`CommonActivatableWidgetContainerBase.ClearWidgets` _pausestack)
      (`WidgetBlueprintLibrary.SetInputMode_GameOnly` _returnvalue)
      (set `PlayerController.bShowMouseCursor` false _returnvalue)
      (`GameplayStatics.SetGamePaused` false)
      (`AudioComponent.SetPaused` (`self.Sounds`) false))))

(event `Apply Brightness`
  (`/Game/MyStuff/Blueprints/GI_Puzzle.ApplyBrightness` (`self.GAMe Instance`)))

(event `OpenSpeech`
  (params (RowName :type String))
  (`/Game/MyStuff/UI/WBP_Monologue.StartSpeech` (`self.SpeechUi`) RowName))

(event `self.ReceiveEndPlay`
  (params (EndPlayReason :type "EEndPlayReason Enum" :default "Destroyed")))

(fn `setUpUI`
  (bind _returnvalue (`|CreateWidget` "/Game/MyStuff/UI/WBP_GameUI.WBP_GameUI_C"))
  (bind _output_get (set `self.GameUI` _returnvalue))
  (`UserWidget.AddToViewport` _output_get 0)
  (`CommonActivatableWidgetContainerBase.BP_AddWidget` (`/Game/MyStuff/UI/WBP_GameUI.GameplayStack` _output_get) "/Game/MyStuff/UI/WBP_GameplayUi.WBP_GameplayUi_C")
  (bind _returnvalue_2 (`CommonActivatableWidgetContainerBase.BP_AddWidget` (`/Game/MyStuff/UI/WBP_GameUI.Dialogue` _output_get) "/Game/MyStuff/UI/WBP_Monologue.WBP_Monologue_C"))
  (set `self.SpeechUi` _returnvalue_2))

(fn `UserConstructionScript`)