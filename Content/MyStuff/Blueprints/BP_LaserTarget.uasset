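; BP_LaserTarget is a powerable target actor that drives an assigned Level Sequence when its power state changes.
; SetPower plays the sequence forward when powered and in reverse when power is lost.
; A pair of DoOnce gates, each reset by the opposite direction, stops repeated calls with the same state from retriggering playback.
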(event `/Game/MyStuff/Blueprints/Interfaces/BPI_EnergyReceiver.SetPower`
  (params (GetPowered :type Boolean))
  (bind _levelsequence (`self.LevelSequence`))
  (bind _levelsequence_2 (`self.LevelSequence`))
  (if GetPowered
    (`/Engine/EditorBlueprintResources/StandardMacros.DoOnce` false :!label _label
      (:`Completed`
        (`/Engine/EditorBlueprintResources/StandardMacros.IsValid` _levelsequence_2
          (:`Is Valid`
            (`MovieSceneSequencePlayer.Play` (`LevelSequenceActor.SequencePlayer` _levelsequence_2))
            (`self.ResetReverse`)))))
    (else
      (`/Engine/EditorBlueprintResources/StandardMacros.DoOnce` false :!label _label_2
        (:`Completed`
          (`/Engine/EditorBlueprintResources/StandardMacros.IsValid` _levelsequence
            (:`Is Valid`
              (`MovieSceneSequencePlayer.PlayReverse` (`LevelSequenceActor.SequencePlayer` _levelsequence))
              (`self.ResetForward`))))))))

(event `ResetForward`
  (goto _label :!via `Reset`))

(event `ResetReverse`
  (goto _label_2 :!via `Reset`))

(fn `UserConstructionScript`)