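; Riddle tracker that keeps a running count of sacrifice answers and triggers the riddle's completion when the count hits the required value.
; Correct and Wrong events both add their passed amount to the count, but only Correct compares it against the target.
; On a match, a DoOnce sends the "end draws near" message, opens the riddle speech through BP_Gamemode_Base and plays a monster call sound.
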(event `self.ReceiveBeginPlay`
  (set `self.Number` 0))

(event `/Game/MyStuff/Blueprints/Interfaces/BPI_RiddleTrue.Correct`
  (params (Yes :type Integer))
  (set `self.Number` (+ (`self.Number`) Yes))
  (if (== (`self.Number`) (`self.Right Sacrifce`))
    (`KismetSystemLibrary.PrintText` "")
    (`/Engine/EditorBlueprintResources/StandardMacros.DoOnce` false
      (:`Completed`
        (message `/Game/MyStuff/Blueprints/Interfaces/BPI_UltimateTracker.TheEnddrawsnear` (`self.Target`) 0)
        (bind _asbp_gamemode_base (cast `/Game/MyStuff/Blueprints/BP_Gamemode_Base` (`GameplayStatics.GetGameMode`)))
        (`/Game/MyStuff/Blueprints/BP_Gamemode_Base.OpenSpeech` _asbp_gamemode_base "riddle")
        (`GameplayStatics.PlaySound2D` "/Game/MyStuff/Sounds/god/creature-abstract-huge-monster-call-communicate-01.creature-abstract-huge-monster-call-communicate-01" 1.0 1.0 0.0 null null)))))

(event `/Game/MyStuff/Blueprints/Interfaces/BPI_RiddleTrue.Wrong`
  (params (Nope :type Integer))
  (set `self.Number` (+ (`self.Number`) Nope)))

(fn `UserConstructionScript`)