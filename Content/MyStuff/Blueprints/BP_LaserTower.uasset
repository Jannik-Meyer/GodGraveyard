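; BP_LaserTower is an interactable, possessable tower that the player rotates to aim an energy laser at receivers.
; Interacting smooth-possesses it, swapping in its input context for yaw aiming and a back action returning to the previous pawn.
; When self-powered, it line-traces each tick, sets the laser effect's endpoint, and toggles power on the hit BPI_EnergyReceiver actor.
; Its own SetPower event only prints the received value.
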(event `self.ReceiveBeginPlay`
  (`self.SetupVariables`))

(event `self.ReceiveTick`
  (params (DeltaSeconds :type "Float (single-precision)"))
  (if (`self.SelfPowered`)
    (`self.ShootLaser`)))

(event `/Game/MyStuff/Blueprints/Interfaces/BPI_Puzzle.SetHighlight`
  (params (On :type Boolean))
  (if On
    (`MeshComponent.SetOverlayMaterial` (`self.LaserTower_Cube`) "/Game/MyStuff/Materials/Postprocess/NewFolder/M_Moving_Pattern.M_Moving_Pattern")
    (`MeshComponent.SetOverlayMaterial` (`self.LaserTower_Cube_001`) "/Game/MyStuff/Materials/Postprocess/NewFolder/M_Moving_Pattern.M_Moving_Pattern")
    (else
      (`MeshComponent.SetOverlayMaterial` (`self.LaserTower_Cube`) null)
      (`MeshComponent.SetOverlayMaterial` (`self.LaserTower_Cube_001`) null))))

(event `SetupVariables`
  (bind _asbp_gamemode_base (cast `/Game/MyStuff/Blueprints/BP_Gamemode_Base` (`GameplayStatics.GetGameMode`)))
  (set `self.GameMode` _asbp_gamemode_base))

(event `/Game/MyStuff/Blueprints/Interfaces/BPI_Puzzle.Interact`
  (params (lastPossessed :type "Pawn Object Reference"))
  (bind _output_get (set `self.Last Possessed` lastPossessed))
  (`self.DisableInput` _output_get null)
  (`/Game/MyStuff/Blueprints/BP_MacroLibrary.MySmoothPosess` self 1.0
    (:`out`
      (`self.EnableInput` (`self.Last Possessed`) null))))

(event `self.ReceivePossessed`
  (params (NewController :type "Controller Object Reference"))
  (`Widget.SetVisibility` (`/Game/MyStuff/Blueprints/BP_Gamemode_Base.GameUI` (`self.GameMode`)) "Collapsed")
  (`EnhancedInputSubsystemInterface.AddMappingContext` (pcsubsystem `EnhancedInputLocalPlayerSubsystem` (`GameplayStatics.GetPlayerController` 0)) "/Game/MyStuff/Input/LaserTower/IMC_LaserTower.IMC_LaserTower" 0 (struct)))

(event `self.ReceiveUnpossessed`
  (params (OldController :type "Controller Object Reference"))
  (`EnhancedInputSubsystemInterface.RemoveMappingContext` (pcsubsystem `EnhancedInputLocalPlayerSubsystem` (`GameplayStatics.GetPlayerController` 0)) "/Game/MyStuff/Input/LaserTower/IMC_LaserTower.IMC_LaserTower" (struct)))

(event `ExitTower`
  (`self.DisableInput` null)
  (`/Game/MyStuff/Blueprints/BP_MacroLibrary.MySmoothPosess` (`self.Last Possessed`) 1.0
    (:`out`
      (`self.EnableInput` null))))

(event `ShootLaser`
  (bind _laserarrow (`self.LaserArrow`))
  (bind _otherreceiver (`self.OtherReceiver`))
  (bind _returnvalue (`SceneComponent.K2_GetComponentLocation` _laserarrow))
  (bind _returnvalue_2 (+ _returnvalue (* (`SceneComponent.GetForwardVector` _laserarrow) 500.0)))
  (`NiagaraComponent.SetVariableVec3` (`self.Laser`) "EndLoc" _returnvalue_2)
  (bind _outhit (`KismetSystemLibrary.LineTraceSingle` :`Start` _returnvalue :`End` _returnvalue_2 :`TraceChannel` "TraceTypeQuery1" :`DrawDebugType` "ForOneFrame"))
  (bind (_bblockinghit _binitialoverlap _time _distance _location _impactpoint _normal _impactnormal _physmat _hitactor) (`GameplayStatics.BreakHitResult` _outhit))
  (if _bblockinghit
    (`NiagaraComponent.SetVariableVec3` (`self.Laser`) "EndLoc" _location)
    (if (`KismetSystemLibrary.DoesImplementInterface` _hitactor "/Game/MyStuff/Blueprints/Interfaces/BPI_EnergyReceiver.BPI_EnergyReceiver_C")
      (bind _output_get (set `self.OtherReceiver` _hitactor))
      (message `/Game/MyStuff/Blueprints/Interfaces/BPI_EnergyReceiver.SetPower` _output_get true)
      (else
        (`/Engine/EditorBlueprintResources/StandardMacros.IsValid` _otherreceiver :!label _label
          (:`Is Valid`
            (message `/Game/MyStuff/Blueprints/Interfaces/BPI_EnergyReceiver.SetPower` _otherreceiver false)
            (set `self.OtherReceiver` null)))))
    (else
      (goto _label))))

(event `/Game/MyStuff/Blueprints/Interfaces/BPI_EnergyReceiver.SetPower`
  (params (GetPowered :type Boolean))
  (`KismetSystemLibrary.PrintString` (`KismetStringLibrary.Conv_BoolToString` GetPowered)))

(event `EnhancedInput|/Game/MyStuff/Input/IA_Look`
  (params (ActionValue :type "Vector2D Structure") (ElapsedSeconds :type "Float (double-precision)") (TriggeredSeconds :type "Float (double-precision)") (InputAction :type "InputAction Object Reference" :default "/Game/MyStuff/Input/IA_Look.IA_Look"))
  (:`Triggered`
    (`SceneComponent.K2_AddRelativeRotation` (`self.LaserTower_Cube_001`) (`KismetMathLibrary.MakeRotator` 0.0 0.0 ActionValue_X) false false)))

(event `EnhancedInput|/Game/MyStuff/Input/Keypad/IA_Back`
  (params (ActionValue :type Boolean) (ElapsedSeconds :type "Float (double-precision)") (TriggeredSeconds :type "Float (double-precision)") (InputAction :type "InputAction Object Reference" :default "/Game/MyStuff/Input/Keypad/IA_Back.IA_Back"))
  (:`Started`
    (`self.ExitTower`)))

(fn `Interactable`
  (returns (Interactable :type Boolean))
  (return true))

(fn `UserConstructionScript`
  (if (`self.SelfPowered`)
    (`self.ShootLaser`)
    (`ActorComponent.SetAutoActivate` (`self.Laser`) true)))