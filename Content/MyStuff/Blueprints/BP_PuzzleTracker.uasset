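; BP_PuzzleTracker keeps a running total for a sacrifice puzzle and triggers the end-is-near sequence.
; ClosertoEnd and FurtherFromeNd add right and wrong sacrifice values to Number, which starts at zero.
; ClosertoEnd compares the new total to the incoming value, so it passes only when the prior total was zero.
; A DoOnce then calls TheEnddrawsnearMessage and opens the "sacrifice" speech through BP_Gamemode_Base.
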(event `self.ReceiveBeginPlay`
  (set `self.Number` 0))

(event `/Game/MyStuff/Blueprints/BPI_Sacrifices.ClosertoEnd`
  (params (RightSacrifce :type Integer))
  (set `self.Number` (+ (`self.Number`) RightSacrifce))
  (if (== (`self.Number`) (`self.Right Sacrifce`))
    (`KismetSystemLibrary.PrintText` "")
    (`/Engine/EditorBlueprintResources/StandardMacros.DoOnce` false
      (:`Completed`
        (message `/Game/MyStuff/Blueprints/Interfaces/BPI_UltimateTracker.TheEnddrawsnear` (`self.Target`) 0)
        (bind _asbp_gamemode_base (cast `/Game/MyStuff/Blueprints/BP_Gamemode_Base` (`GameplayStatics.GetGameMode`)))
        (`/Game/MyStuff/Blueprints/BP_Gamemode_Base.OpenSpeech` _asbp_gamemode_base "sacrifice")))))

(event `/Game/MyStuff/Blueprints/BPI_Sacrifices.FurtherFromeNd`
  (params (`wrong sacrifive` :type Integer))
  (set `self.Number` (+ (`self.Number`) `wrong sacrifive`)))

(fn `UserConstructionScript`)