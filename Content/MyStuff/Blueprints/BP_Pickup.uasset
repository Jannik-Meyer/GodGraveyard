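; BP_Pickup is an interactable, possessable item that the player can pick up, drop, highlight with an outline overlay and inspect.
; Interact hands it to BP_Player when the hand slot is empty; Drop detaches it and restores collision.
; Inspection possesses the pickup, matches the player's camera and animates the mesh to the inspect point, where IMC_Pickup input rotates it.
; Backing out eases the original transform back, then repossesses the player.
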(event `self.ReceiveBeginPlay`
  (set `self.OriginalRelativeSceneTransform` (`SceneComponent.GetRelativeTransform` (`self.Scene`))))

(event `/Game/MyStuff/Blueprints/Interfaces/BPI_Puzzle.SetHighlight`
  (params (On :type Boolean))
  (`MeshComponent.SetOverlayMaterial` (`self.Object`) (select `bool` On :`true` "/Game/MyStuff/Materials/Postprocess/NewFolder/M_Outline.M_Outline" :!type "MaterialInterface Object Reference")))

(event `/Game/MyStuff/Blueprints/Interfaces/BPI_Puzzle.Interact`
  (params (lastPossessed :type "Pawn Object Reference"))
  (bind _asbp_player (cast `/Game/MyStuff/Blueprints/BP_Player` lastPossessed))
  (bind _output_get (set `self.Player` _asbp_player))
  (`/Engine/EditorBlueprintResources/StandardMacros.IsValid` (`/Game/MyStuff/Blueprints/BP_Player.HandSlot` _output_get)
    (:`Is Not Valid`
      (`/Game/MyStuff/Blueprints/BP_Player.Pickup Object` _output_get self))))

(event `Drop`
  (params (`New location` :type "Vector Structure") (`New Rotation` :type "Rotator Structure"))
  (`self.K2_DetachFromActor` "KeepWorld")
  (`self.K2_SetActorLocation` `New location`)
  (`self.K2_SetActorRotation` `New Rotation`)
  (`PrimitiveComponent.SetCollisionEnabled` (`self.Object`) "QueryAndPhysics"))

(event `Start Inspect`
  (bind _originalrelativescenetransform_location (`KismetMathLibrary.BreakTransform` (`self.OriginalRelativeSceneTransform`)))
  (bind _camera (`/Game/MyStuff/Blueprints/BP_Player.Camera` (`self.Player`)))
  (`/Game/MyStuff/Blueprints/BP_MacroLibrary.MySmoothPosess` self
    (:`out`
      (`SceneComponent.K2_SetRelativeLocation` (`self.Scene`) (0.0 0.0 10.0) false false)
      (`SceneComponent.K2_SetWorldLocationAndRotation` (`self.Camera`) (`SceneComponent.K2_GetComponentLocation` _camera) (`SceneComponent.K2_GetComponentRotation` _camera) false false)
      (bind (_direction _alpha) (`Timeline|InspectAnim` :!via `PlayFromStart`)
        (:`Update`
          (`SceneComponent.K2_SetRelativeLocation` (`self.Scene`) (`KismetMathLibrary.VLerp` _originalrelativescenetransform_location (`KismetMathLibrary.InverseTransformLocation` (`self.GetTransform`) (`SceneComponent.K2_GetComponentLocation` (`/Game/MyStuff/Blueprints/BP_Player.InspectLoc` (`self.Player`)))) _alpha) false false))))))

(event `Stop Inspect`
  (bind (_originalrelativescenetransform_location _originalrelativescenetransform_rotation) (`KismetMathLibrary.BreakTransform` (`self.OriginalRelativeSceneTransform`)))
  (if (not (or (`TimelineComponent.IsPlaying` (`self.StopInspectAnim`)) (`TimelineComponent.IsPlaying` (`self.InspectAnim`))))
    (bind (_direction _alpha) (`Timeline|StopInspectAnim` :!via `PlayFromStart`)
      (:`Update`
        (`SceneComponent.K2_SetRelativeLocation` (`self.Scene`) (`KismetMathLibrary.VLerp` (`KismetMathLibrary.InverseTransformLocation` (`self.GetTransform`) (`SceneComponent.K2_GetComponentLocation` (`/Game/MyStuff/Blueprints/BP_Player.InspectLoc` (`self.Player`)))) _originalrelativescenetransform_location _alpha) false false)
        (`SceneComponent.K2_SetRelativeRotation` (`self.Scene`) (`KismetMathLibrary.RLerp` (`SceneComponent.RelativeRotation` (`self.Scene`)) _originalrelativescenetransform_rotation _alpha) false false))
      (:`Finished`
        (`/Game/MyStuff/Blueprints/BP_MacroLibrary.MySmoothPosess` (`self.Player`))))))

(event `self.ReceivePossessed`
  (params (NewController :type "Controller Object Reference"))
  (bind _returnvalue (pcsubsystem `EnhancedInputLocalPlayerSubsystem` (`GameplayStatics.GetPlayerController` 0)))
  (`/Engine/EditorBlueprintResources/StandardMacros.IsValid` _returnvalue
    (:`Is Valid`
      (`EnhancedInputSubsystemInterface.AddMappingContext` _returnvalue "/Game/MyStuff/Input/InspectPickup/IMC_Pickup.IMC_Pickup" 0 (struct)))))

(event `self.ReceiveUnpossessed`
  (params (OldController :type "Controller Object Reference"))
  (bind _returnvalue (pcsubsystem `EnhancedInputLocalPlayerSubsystem` (`GameplayStatics.GetPlayerController` 0)))
  (`/Engine/EditorBlueprintResources/StandardMacros.IsValid` _returnvalue
    (:`Is Valid`
      (`EnhancedInputSubsystemInterface.RemoveMappingContext` _returnvalue "/Game/MyStuff/Input/InspectPickup/IMC_Pickup.IMC_Pickup" (struct)))))

(event `EnhancedInput|/Game/MyStuff/Input/Keypad/IA_Back`
  (params (ActionValue :type Boolean) (ElapsedSeconds :type "Float (double-precision)") (TriggeredSeconds :type "Float (double-precision)") (InputAction :type "InputAction Object Reference" :default "/Game/MyStuff/Input/Keypad/IA_Back.IA_Back"))
  (:`Started`
    (`self.Stop Inspect`)))

(event `EnhancedInput|/Game/MyStuff/Input/IA_Look`
  (params (ActionValue :type "Vector2D Structure") (ElapsedSeconds :type "Float (double-precision)") (TriggeredSeconds :type "Float (double-precision)") (InputAction :type "InputAction Object Reference" :default "/Game/MyStuff/Input/IA_Look.IA_Look"))
  (:`Triggered`
    (`SceneComponent.K2_AddWorldRotation` (`self.Scene`) (`KismetMathLibrary.MakeRotator` 0.0 ActionValue_Y ActionValue_X) false false)))

(fn `Interactable`
  (returns (Interactable :type Boolean))
  (return true))

(fn `UserConstructionScript`)