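; Component that detects the puzzle interactable the owning pawn is looking at and highlights it.
; Each tick it sphere traces a short distance along the camera's forward vector, accepting only BPI_Puzzle actors while the pawn is controlled.
; It moves the highlight via SetHighlightMessage when the target changes and clears it otherwise.
; CanInteract exposes the current target and whether it is valid.
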(event `self.ReceiveTick`
  (params (DeltaSeconds :type "Float (single-precision)"))
  (bind _camera (`self.Camera`))
  (bind _returnvalue (`SceneComponent.K2_GetComponentLocation` _camera))
  (bind _outhit (`KismetSystemLibrary.SphereTraceSingle` _returnvalue (+ _returnvalue (* (`SceneComponent.GetForwardVector` _camera) 250.0)) 5.0 "TraceTypeQuery1"))
  (bind (_bblockinghit _binitialoverlap _time _distance _location _impactpoint _normal _impactnormal _physmat _hitactor) (`GameplayStatics.BreakHitResult` _outhit))
  (if (and (`KismetSystemLibrary.DoesImplementInterface` _hitactor "/Game/MyStuff/Blueprints/Interfaces/BPI_Puzzle.BPI_Puzzle_C") (`Pawn.IsPawnControlled` (cast `Pawn` (`self.GetOwner`) :!pure true)))
    (if (not (== _hitactor (`self.CurrentInteractable`)))
      ;[1 1 1] highlight
      (message `/Game/MyStuff/Blueprints/Interfaces/BPI_Puzzle.SetHighlight` (`self.CurrentInteractable`) false)
      (bind _output_get (set `self.CurrentInteractable` _hitactor))
      (message `/Game/MyStuff/Blueprints/Interfaces/BPI_Puzzle.SetHighlight` _output_get true))
    (else
      ;[1 1 1] deselct Highlight
      (message `/Game/MyStuff/Blueprints/Interfaces/BPI_Puzzle.SetHighlight` (`self.CurrentInteractable`) false)
      (set `self.CurrentInteractable` null))))

(fn `CanInteract`
  (returns (CanInteract :type Boolean) (CurrentInteractable :type "Actor Object Reference"))
  (bind _currentinteractable (`self.CurrentInteractable`))
  (return (`KismetSystemLibrary.IsValid` _currentinteractable) _currentinteractable))