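; BP_FinalTracker counts progress toward the game's ending, revealing eyes and updating the god's dialogue as it advances.
; Each TheEnddrawsnear call increments a counter, makes that eye visible and collidable, and copies the matching line to BP_GodTalks.
; The increment precedes indexing, so the event skips array index zero if the counter starts there.
; At the third step, after a delay, it opens the game mode's "end" speech and sets BP_GodTalks' End flag.
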(event `/Game/MyStuff/Blueprints/Interfaces/BPI_UltimateTracker.TheEnddrawsnear`
  (params (Closer :type Integer))
  (bind _output (`|GetArrayItem` (`self.Eyes`) (`self.CLosetoEnd`)))
  (`/Engine/EditorBlueprintResources/StandardMacros.IncrementInt` (`self.CLosetoEnd`)
    (:`  `
      (`KismetSystemLibrary.PrintString` "Hello")
      (`SceneComponent.SetVisibility` _output true false)
      (`PrimitiveComponent.SetCollisionEnabled` _output "QueryAndPhysics")
      (bind _asbp_god_talks (cast `/Game/MyStuff/Blueprints/BP_GodTalks` (`self.GodTalks`)))
      (set `/Game/MyStuff/Blueprints/BP_GodTalks.Dialogue` (`|GetArrayItem` (`self.GosWords`) (`self.CLosetoEnd`)) _asbp_god_talks)
      (if (== 3 (`self.CLosetoEnd`))
        (`KismetSystemLibrary.Delay` 9.0)
        (bind _asbp_gamemode_base (cast `/Game/MyStuff/Blueprints/BP_Gamemode_Base` (`GameplayStatics.GetGameMode`)))
        (`/Game/MyStuff/Blueprints/BP_Gamemode_Base.OpenSpeech` _asbp_gamemode_base "end")
        (bind _asbp_god_talks_2 (cast `/Game/MyStuff/Blueprints/BP_GodTalks` (`self.GodTalks`)))
        (set `/Game/MyStuff/Blueprints/BP_GodTalks.End` true _asbp_god_talks_2)))))

(event `self.ReceiveBeginPlay`
  (set `self.Eyes` (`|MakeArray` (`self.eye`) (`self.eye1`) (`self.eye2`) (`self.eye3`))))

(fn `UserConstructionScript`)