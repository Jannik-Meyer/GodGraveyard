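; BP_DialPuzzle is an interactable three-dial combination puzzle with two successive codes and an outline highlight.
; RotatorCallUp turns the given dial by a fixed yaw step, then CheckCode compares that dial's yaw to its code entry within a tolerance.
; Solving the first code plays an attached Song event and swaps in the second.
; Solving that sends TheEnddrawsnear message once, opens "song" speech through the game mode and plays a creature call.
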(event `/Game/MyStuff/Blueprints/Interfaces/BPI_Puzzle.Interact`
  (params (lastPossessed :type "Pawn Object Reference")))

(event `/Game/MyStuff/Blueprints/Interfaces/BPI_Rotator.Rotator Call Up`
  (params (Component :type "PrimitiveComponent Object Reference"))
  (bind _output_get (set `self.Component` Component))
  (`self.RotateDial` _output_get))

(event `/Game/MyStuff/Blueprints/Interfaces/BPI_Puzzle.SetHighlight`
  (params (On :type Boolean))
  (bind _dial (`self.Dial`))
  (if On
    (`MeshComponent.SetOverlayMaterial` _dial "/Game/MyStuff/Materials/Postprocess/NewFolder/M_Outline.M_Outline")
    (`MeshComponent.SetOverlayMaterial` (`self.Dial2`) "/Game/MyStuff/Materials/Postprocess/NewFolder/M_Outline.M_Outline")
    (`MeshComponent.SetOverlayMaterial` (`self.Dial1`) "/Game/MyStuff/Materials/Postprocess/NewFolder/M_Outline.M_Outline")
    (else
      (`MeshComponent.SetOverlayMaterial` _dial null)
      (`MeshComponent.SetOverlayMaterial` (`self.Dial1`) null)
      (`MeshComponent.SetOverlayMaterial` (`self.Dial2`) null))))

(fn `CheckCode`
  (params (Component :type "PrimitiveComponent Object Reference"))
  (locals (`Selected Mesh` :type Integer) (LocalFailed :type Boolean))
  (bind (_relativerotation_roll _relativerotation_pitch _relativerotation_yaw) (`KismetMathLibrary.BreakRotator` (`SceneComponent.RelativeRotation` Component)))
  (if (== Component (`self.Dial1`))
    (set `local.Selected Mesh` 0)
    (`KismetArrayLibrary.Array_Set` (`self.CodeIsGood`) (`local.Selected Mesh`) (`KismetMathLibrary.NearlyEqual_FloatFloat` (`|GetArrayItem` (`self.Code`) (`local.Selected Mesh`)) _relativerotation_yaw 1.0) :!label _label)
    (for _array_element (`self.CodeIsGood`)
      (if (not _array_element)
        (set `local.LocalFailed` true)
        (break)))
    (if (not (`local.LocalFailed`))
      (`KismetSystemLibrary.PrintString` "")
      (if (`self.FinalCode`)
        (if (not (`self.Condition`))
          (`KismetSystemLibrary.PrintString` "")
          (`/Engine/EditorBlueprintResources/StandardMacros.DoOnce` false
            (:`Completed`
              (message `/Game/MyStuff/Blueprints/Interfaces/BPI_UltimateTracker.TheEnddrawsnear` (`self.Target`) 0)
              (set `self.Condition` true)
              (bind _asbp_gamemode_base (cast `/Game/MyStuff/Blueprints/BP_Gamemode_Base` (`GameplayStatics.GetGameMode`)))
              (`/Game/MyStuff/Blueprints/BP_Gamemode_Base.OpenSpeech` _asbp_gamemode_base "song")
              (`GameplayStatics.PlaySound2D` "/Game/MyStuff/Sounds/god/creature-abstract-huge-monster-call-communicate-01.creature-abstract-huge-monster-call-communicate-01" 1.0 1.0 0.0 null null))))
        (else
          (set `self.Code` (`self.SecondCode`))
          (set `self.FinalCode` true)
          (set `self.CodeIsGood` (`|MakeArray` false false false))
          (`FMODBlueprintStatics.PlayEventAttached` "/Game/FMOD/Events/song/song.song" (`self.Dial`) "None" (0.0 0.0 0.0) "KeepRelativeOffset" false true false))))
    (elif (== Component (`self.Dial`))
      (set `local.Selected Mesh` 1)
      (goto _label)
      (elif (== Component (`self.Dial2`))
        (set `local.Selected Mesh` 2)
        (goto _label)))))

(fn `Interactable`
  (returns (Interactable :type Boolean))
  (return true))

(fn `ResetForward`)

(fn `ResetReverse`)

(fn `RotateDial`
  (params (Component :type "PrimitiveComponent Object Reference") (`Rotate Left` :type Boolean :default false))
  (if `Rotate Left`
    (`SceneComponent.K2_AddRelativeRotation` Component (`KismetMathLibrary.MakeRotator` 0.0 0.0 (* (`self.RotateValue`) -1.0)) false false)
    (else
      (`SceneComponent.K2_AddRelativeRotation` Component (`KismetMathLibrary.MakeRotator` 0.0 0.0 (`self.RotateValue`)) false false)))
  (`KismetSystemLibrary.PrintString` "")
  (`self.CheckCode` Component))

(fn `UserConstructionScript`)