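; Interactable keypad pawn: the player enters a code, and a correct one locks out further interaction and plays a sequence.
; Interacting smoothly possesses the keypad, which adds its input mapping context and hides the game UI.
; Directional input moves a wrapping selection across the button grid; confirming animates a press and edits or checks the code, flashing red on failure.
; Exiting repositions the player via a downward trace and blends possession back.
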(event `self.ReceiveBeginPlay`
  (`self.SetupVariables`))

(event `SetupVariables`
  (bind _asbp_gamemode_base (cast `/Game/MyStuff/Blueprints/BP_Gamemode_Base` (`GameplayStatics.GetGameMode`)))
  (set `self.GameMode` _asbp_gamemode_base))

(event `/Game/MyStuff/Blueprints/Interfaces/BPI_Puzzle.SetHighlight`
  (params (On :type Boolean))
  ;[1 1 1] set high
  (if On
    (`MeshComponent.SetOverlayMaterial` (`self.KeypadBase`) "/Game/MyStuff/Materials/Postprocess/NewFolder/M_Moving_Pattern.M_Moving_Pattern")
    (else
      (`MeshComponent.SetOverlayMaterial` (`self.KeypadBase`) null))))

(event `/Game/MyStuff/Blueprints/Interfaces/BPI_Puzzle.Interact`
  (params (lastPossessed :type "Pawn Object Reference"))
  ;[1 1 1] interact
  (`|ExecutionSequence`
    (:`then_0`
      (`/Game/MyStuff/Blueprints/BP_MacroLibrary.MySmoothPosess` self 2.0
        (:`out`
          (bind _output_get (set `self.CurrentButton` 0))
          (`self.SetButtonSelected` _output_get true))))
    (:`then_1`
      (bind _output_get_2 (set `self.Last Possessed` lastPossessed))
      (bind _asbp_player (cast `/Game/MyStuff/Blueprints/BP_Player` _output_get_2))
      (set `/Game/MyStuff/Blueprints/BP_Player.CanMove` false _asbp_player))))

(event `self.ReceivePossessed`
  (params (NewController :type "Controller Object Reference"))
  ;[1 1 1] possess/unpossess
  (`EnhancedInputSubsystemInterface.AddMappingContext` (pcsubsystem `EnhancedInputLocalPlayerSubsystem` (`GameplayStatics.GetPlayerController` 0)) "/Game/MyStuff/Input/Keypad/IMC_Keypad.IMC_Keypad" 0 (struct))
  (`Widget.SetVisibility` (`/Game/MyStuff/Blueprints/BP_Gamemode_Base.GameUI` (`self.GameMode`)) "Collapsed"))

(event `self.ReceiveUnpossessed`
  (params (OldController :type "Controller Object Reference"))
  ;[1 1 1] possess/unpossess
  (`EnhancedInputSubsystemInterface.RemoveMappingContext` (pcsubsystem `EnhancedInputLocalPlayerSubsystem` (`GameplayStatics.GetPlayerController` 0)) "/Game/MyStuff/Input/Keypad/IMC_Keypad.IMC_Keypad" (struct)))

(event `ExitKeypad`
  (`self.Reposition Player`)
  (set `self.canSelect` false)
  (`/Game/MyStuff/Blueprints/BP_MacroLibrary.MySmoothPosess` (`self.Last Possessed`) 1.5
    (:`out`
      (set `self.canSelect` true)
      (`self.SetButtonSelected` (`self.CurrentButton`)))))

(event `SetButtonSelected`
  (params (Position :type Integer) (Select :type Boolean))
  ;[1 1 1] set button select
  (`/Game/MyStuff/Blueprints/BP_KeypadButton.SetSelected` (`|GetArrayItem` (`self.buttonList`) Position) Select))

(event `AnimatePress`
  ;[1 1 1] Comment
  (`/Engine/EditorBlueprintResources/StandardMacros.IsValid` (`self.LastPressedButton`)
    (:`Is Valid`
      (`SceneComponent.K2_SetRelativeLocation` (`self.LastPressedButton`) (0.0 0.0 0.0) false false))
    (:`Is Not Valid`
      _))
  (set `self.LastPressedButton` (`|GetArrayItem` (`self.buttonList`) (`self.CurrentButton`)))
  (`TimelineComponent.SetPlayRate` (`self.ButtonPress`) 4.0)
  (bind (_direction _alpha) (`Timeline|ButtonPress` :!via `PlayFromStart`)
    (:`Update`
      (`SceneComponent.K2_SetRelativeLocation` (`self.LastPressedButton`) (`KismetMathLibrary.MakeVector` 0.0 (`KismetMathLibrary.Lerp` 0.0 -2.0 _alpha)) false false))))

(event `Reposition Player`
  (bind _returnvalue (`SceneComponent.K2_GetComponentLocation` (`self.PlayerPosition`)))
  ;[1 1 1] Comment
  (bind _outhit (`KismetSystemLibrary.LineTraceSingle` _returnvalue (- _returnvalue (0.0 0.0 250.0)) "TraceTypeQuery1"))
  (`self.K2_SetActorLocationAndRotation` (`self.Last Possessed`) (+ (`.Location` (`GameplayStatics.BreakHitResult` _outhit)) (0.0 0.0 88.0)) (`SceneComponent.K2_GetComponentRotation` (`self.PlayerPosition`)) false false))

(event `EnhancedInput|/Game/MyStuff/Input/Keypad/IA_Back`
  (params (ActionValue :type Boolean) (ElapsedSeconds :type "Float (double-precision)") (TriggeredSeconds :type "Float (double-precision)") (InputAction :type "InputAction Object Reference" :default "/Game/MyStuff/Input/Keypad/IA_Back.IA_Back"))
  (:`Started`
    (if (`self.canSelect`)
      (`self.ExitKeypad`))))

(event `EnhancedInput|/Game/MyStuff/Input/Keypad/IA_Right`
  (params (ActionValue :type Boolean) (ElapsedSeconds :type "Float (double-precision)") (TriggeredSeconds :type "Float (double-precision)") (InputAction :type "InputAction Object Reference" :default "/Game/MyStuff/Input/Keypad/IA_Right.IA_Right"))
  ;[1 1 1] right input
  (:`Started`
    (if (`self.canSelect`)
      (`self.SetButtonSelected` (`self.CurrentButton`))
      (bind _result (`/Engine/EditorBlueprintResources/StandardMacros.IncrementInt` (`self.CurrentButton`))
        (:`  `
          (if (not (< _result (`KismetArrayLibrary.Array_Length` (`self.buttonList`))))
            (set `self.CurrentButton` 0))
          (`self.SetButtonSelected` (`self.CurrentButton`) true))))))

(event `EnhancedInput|/Game/MyStuff/Input/Keypad/IA_Left`
  (params (ActionValue :type Boolean) (ElapsedSeconds :type "Float (double-precision)") (TriggeredSeconds :type "Float (double-precision)") (InputAction :type "InputAction Object Reference" :default "/Game/MyStuff/Input/Keypad/IA_Left.IA_Left"))
  ;[1 1 1] left
  (:`Started`
    (if (`self.canSelect`)
      (`self.SetButtonSelected` (`self.CurrentButton`))
      (bind _result (`/Engine/EditorBlueprintResources/StandardMacros.DecrementInt` (`self.CurrentButton`))
        (:`  `
          (if (not (> _result -1))
            (bind _result_2 (`/Engine/EditorBlueprintResources/StandardMacros.DecrementInt` (`KismetArrayLibrary.Array_Length` (`self.buttonList`)))
              (:`  `
                (set `self.CurrentButton` _result_2))))
          (`self.SetButtonSelected` (`self.CurrentButton`) true))))))

(event `EnhancedInput|/Game/MyStuff/Input/Keypad/IA_down`
  (params (ActionValue :type Boolean) (ElapsedSeconds :type "Float (double-precision)") (TriggeredSeconds :type "Float (double-precision)") (InputAction :type "InputAction Object Reference" :default "/Game/MyStuff/Input/Keypad/IA_down.IA_down"))
  ;[1 1 1] down
  (:`Started`
    (if (`self.canSelect`)
      (`self.SetButtonSelected` (`self.CurrentButton`))
      (bind _output_get (set `self.CurrentButton` (+ (`self.CurrentButton`) (`self.buttonsPerRow`))))
      (if (not (< _output_get (`KismetArrayLibrary.Array_Length` (`self.buttonList`))))
        (set `self.CurrentButton` (- (`self.CurrentButton`) (`KismetArrayLibrary.Array_Length` (`self.buttonList`)))))
      (`self.SetButtonSelected` (`self.CurrentButton`) true))))

(event `EnhancedInput|/Game/MyStuff/Input/Keypad/IA_Up`
  (params (ActionValue :type Boolean) (ElapsedSeconds :type "Float (double-precision)") (TriggeredSeconds :type "Float (double-precision)") (InputAction :type "InputAction Object Reference" :default "/Game/MyStuff/Input/Keypad/IA_Up.IA_Up"))
  ;[1 1 1] up
  (:`Started`
    (if (`self.canSelect`)
      (`self.SetButtonSelected` (`self.CurrentButton`))
      (bind _output_get (set `self.CurrentButton` (- (`self.CurrentButton`) (`self.buttonsPerRow`))))
      (if (not (> _output_get -1))
        (set `self.CurrentButton` (+ (`self.CurrentButton`) (`KismetArrayLibrary.Array_Length` (`self.buttonList`)))))
      (`self.SetButtonSelected` (`self.CurrentButton`) true))))

(event `EnhancedInput|/Game/MyStuff/Input/IA_Interact`
  (params (ActionValue :type Boolean) (ElapsedSeconds :type "Float (double-precision)") (TriggeredSeconds :type "Float (double-precision)") (InputAction :type "InputAction Object Reference" :default "/Game/MyStuff/Input/IA_Interact.IA_Interact"))
  (bind _buttoncontent (`/Game/MyStuff/Blueprints/BP_KeypadButton.ButtonContent` (`|GetArrayItem` (`self.buttonList`) (`self.CurrentButton`))))
  (:`Started`
    (if (`self.canSelect`)
      (`self.AnimatePress`)
      (switch `string` _buttoncontent
        (:`Default`
          ;[1 1 1] add number to current code
          (if (< (`KismetStringLibrary.Len` (`self.currentCode`)) (`self.MaxCodeLenghth`))
            (bind _output_get (set `self.currentCode` (`KismetStringLibrary.Concat_StrStr` (`self.currentCode`) _buttoncontent)))
            (`TextRenderComponent.K2_SetText` (`self.Text_CurrentCode`) (`KismetTextLibrary.Conv_StringToText` _output_get))))
        (:`enter`
          (if (`KismetStringLibrary.EqualEqual_StrStr` (`self.currentCode`) (`self.wantedCode`))
            (set `self.isInteractable` false)
            (`TextRenderComponent.SetTextRenderColor` (`self.Text_CurrentCode`) (make `Color` 0 255))
            (`self.ExitKeypad`)
            (`MovieSceneSequencePlayer.Play` (`LevelSequenceActor.SequencePlayer` (`self.SequenceToPlay`)))
            (elif (not (`KismetStringLibrary.EqualEqual_StrStr` (`self.currentCode`)))
              (set `self.canSelect` false)
              (`TextRenderComponent.SetTextRenderColor` (`self.Text_CurrentCode`) (make `Color` 0 0 255))
              (`KismetSystemLibrary.Delay` 1.5)
              (bind _output_get_2 (set `self.currentCode` ""))
              (`TextRenderComponent.K2_SetText` (`self.Text_CurrentCode`) (`KismetTextLibrary.Conv_StringToText` _output_get_2))
              (`TextRenderComponent.SetTextRenderColor` (`self.Text_CurrentCode`) (make `Color` 255 255 255))
              (set `self.canSelect` true))))
        (:`cancel`
          ;[1 1 1] delete
          (bind _output_get_3 (set `self.currentCode` ""))
          (`TextRenderComponent.K2_SetText` (`self.Text_CurrentCode`) (`KismetTextLibrary.Conv_StringToText` _output_get_3)))))))

(fn `Interactable`
  (returns (Interactable :type Boolean))
  (return (`self.isInteractable`)))

(fn `UserConstructionScript`
  (set `self.buttonList` (`|MakeArray` (`self.1`) (`self.2`) (`self.3`) (`self.4`) (`self.5`) (`self.6`) (`self.7`) (`self.8`) (`self.9`) (`self.exit`) (`self.0`) (`self.enter`))))