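; First-person player character with Enhanced Input movement, look, sprint, flashlight, pause and interaction through a CheckForInteractables component.
; A velocity-scaled HeadWobble timeline bobs the camera and triggers surface-based footstep audio via a downward trace.
; One held object animates into the hand, can be inspected, and drops onto traced upward-facing surfaces.
; Possession toggles the mapping context, destruction notifies the game mode, and crouch input is unwired.
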(event `self.ReceiveBeginPlay`
  (`self.Add Mapping Context` false)
  (`self.SetUpCamera`)
  (`self.HeadWobble`)
  (`self.SetUpVariable`))

(event `PlayFootstep`
  (bind _returnvalue (`self.K2_GetActorLocation`))
  (bind _outhit (`KismetSystemLibrary.LineTraceSingle` _returnvalue (+ _returnvalue (* (`KismetMathLibrary.Vector_Down`) 120)) "TraceTypeQuery1"))
  (bind (_bblockinghit _binitialoverlap _time _distance _location _impactpoint _normal _impactnormal _physmat) (`GameplayStatics.BreakHitResult` _outhit))
  (if _bblockinghit
    (`FMODBlueprintStatics.PlayEventAtLocation` (select `EPhysicalSurface` (`PhysicalMaterial.SurfaceType` _physmat) :`SurfaceType1` "/Game/FMOD/Events/Ground/SAnd.SAnd" :`SurfaceType2` "/Game/FMOD/Events/Ground/Stone.Stone" :!type "FMODEvent Object Reference") (`KismetMathLibrary.Conv_VectorToTransform` _location))))

(event `HeadWobble`
  (bind _charactermovement (`self.CharacterMovement`))
  (bind _returnvalue (`KismetMathLibrary.VSizeXY` (`MovementComponent.Velocity` _charactermovement)))
  (bind _returnvalue_2 (`KismetMathLibrary.MapRangeClamped` _returnvalue 0.0 (`CharacterMovementComponent.MaxWalkSpeed` _charactermovement) 0.2 1.0))
  ;[1 1 1] HeadWobble
  (bind (_direction _newtrack_0) (`Timeline|HeadWobblee`)
    (:`Update`
      (`TimelineComponent.SetPlayRate` (`self.HeadWobblee`) (`self.HeadWobbleSpeed`))
      (`SceneComponent.K2_SetRelativeLocation` (`self.Camera`) (`KismetMathLibrary.MakeVector` 0.0 0.0 (* _newtrack_0 (`self.headWobbleAmount`) _returnvalue_2)) false false)
      (set `self.HeadWobbleSpeed` _returnvalue_2))
    (:`Event`
      (if (> _returnvalue 50.0)
        (`self.PlayFootstep`)))))

(event `SetUpVariable`
  (bind _asbp_gamemode_base (cast `/Game/MyStuff/Blueprints/BP_Gamemode_Base` (`GameplayStatics.GetGameMode`)))
  (set `self.GameMode` _asbp_gamemode_base))

(event `Setup Timelines`
  ;[1 1 1] Comment
  (`|ExecutionSequence`
    (:`then_0`
      (`TimelineComponent.SetPlayRate` (`self.DropAnim`) 9.0))
    (:`then_1`
      (`TimelineComponent.SetPlayRate` (`self.PickupAnim`) 9.0))))

(event `MyCrouch`
  ;[1 1 1] crouch
  (set `SpringArmComponent.bEnableCameraLag` true (`self.SpringArm`))
  (`self.Crouch`)
  (`TimelineComponent.SetPlayRate` (`self.CrouchLag`) 3.0)
  (bind (_direction _alpha) (`Timeline|CrouchLag` :!label _label)
    (:`Update`
      (set `SpringArmComponent.CameraLagMaxDistance` (* _alpha 10.0) (`self.SpringArm`)))
    (:`Finished`
      (switch `ETimelineDirection` _direction
        (:`Forward`
          (`self.UndoCrouchLag`)
          (`TimelineComponent.SetPlayRate` (`self.CrouchLag`) 0.7))
        (:`Backward`
          (set `SpringArmComponent.bEnableCameraLag` true (`self.SpringArm`)))))))

(event `UndoCrouchLag`
  ;[1 1 1] crouch
  (goto _label :!via `Reverse`))

(event `self.ReceivePossessed`
  (params (NewController :type "Controller Object Reference"))
  (bind _gamemode (`self.GameMode`))
  ;[1 1 1] possessed
  (`self.Add Mapping Context` false)
  (set `self.CanMove` true)
  (`/Engine/EditorBlueprintResources/StandardMacros.IsValid` _gamemode
    (:`Is Valid`
      (`Widget.SetVisibility` (`/Game/MyStuff/Blueprints/BP_Gamemode_Base.GameUI` _gamemode) "Visible"))))

(event `self.ReceiveUnpossessed`
  (params (OldController :type "Controller Object Reference"))
  ;[1 1 1] unpossessed
  (`self.Add Mapping Context` true)
  (`SceneComponent.SetVisibility` (`self.SpotLight`) false false)
  (`SceneComponent.SetVisibility` (`self.SpotLight1`) false false)
  (`self.SpawnDefaultController`))

(event `self.ReceiveDestroyed`
  ;[1 1 1] destroyed
  (bind _asbp_gamemode_base (cast `/Game/MyStuff/Blueprints/BP_Gamemode_Base` (`GameplayStatics.GetGameMode`)))
  (`/Game/MyStuff/Blueprints/BP_Gamemode_Base.PlayerDied` _asbp_gamemode_base))

(event `Pickup Object`
  (params (ObjectToPickup :type "/Game/MyStuff/Blueprints/BP_Pickup Object Reference"))
  (bind _pickuploc (`self.PickupLoc`))
  (bind (_handslotorigintransfrom_location _handslotorigintransfrom_rotation) (`KismetMathLibrary.BreakTransform` (`self.HandSlotOriginTransfrom`)))
  (bind _output_get (set `self.HandSlot` ObjectToPickup))
  (set `self.HandSlotOriginTransfrom` (`self.GetTransform` _output_get))
  (`PrimitiveComponent.SetCollisionEnabled` (`/Game/MyStuff/Blueprints/BP_Pickup.Object` (`self.HandSlot`)) "NoCollision")
  (bind (_direction _alpha) (`Timeline|PickupAnim` :!via `PlayFromStart`)
    (:`Update`
      (`self.K2_SetActorLocationAndRotation` (`self.HandSlot`) (`KismetMathLibrary.VLerp` _handslotorigintransfrom_location (`SceneComponent.K2_GetComponentLocation` _pickuploc) _alpha) (`KismetMathLibrary.RLerp` _handslotorigintransfrom_rotation (`SceneComponent.RelativeRotation` _pickuploc) _alpha) false false))
    (:`Finished`
      (`self.K2_AttachToComponent` (`self.HandSlot`) (`self.PickupLoc`) "None" "SnapToTarget" "KeepRelative" "KeepRelative" true))))

(event `Drop Object`
  (bind _camera (`self.Camera`))
  (bind _returnvalue (`SceneComponent.K2_GetComponentLocation` _camera))
  (`/Engine/EditorBlueprintResources/StandardMacros.IsValid` (`self.HandSlot`)
    (:`Is Valid`
      (if (not (or (`TimelineComponent.IsPlaying` (`self.PickupAnim`)) (`TimelineComponent.IsPlaying` (`self.DropAnim`))))
        (bind _outhit (`KismetSystemLibrary.LineTraceSingle` _returnvalue (+ _returnvalue (* (`SceneComponent.GetForwardVector` _camera) 250.0)) "TraceTypeQuery1"))
        (bind (_bblockinghit _binitialoverlap _time _distance _location _impactpoint _normal) (`GameplayStatics.BreakHitResult` _outhit))
        (if (and _bblockinghit (> (.z _normal) 0.6))
          (bind (_direction _alpha) (`Timeline|DropAnim` :!via `PlayFromStart`)
            (:`Update`
              (`self.K2_SetActorLocationAndRotation` :`self` (`self.HandSlot`) :`NewLocation` (`KismetMathLibrary.VLerp` (`SceneComponent.K2_GetComponentLocation` (`self.PickupLoc`)) _location _alpha)))
            (:`Finished`
              (`/Game/MyStuff/Blueprints/BP_Pickup.Drop` (`self.HandSlot`) _location (`KismetMathLibrary.MakeRotFromZ` _normal))
              (set `self.HandSlot` null))))))))

(event `EnhancedInput|/Game/MyStuff/Input/IA_Move`
  (params (ActionValue :type "Vector2D Structure") (ElapsedSeconds :type "Float (double-precision)") (TriggeredSeconds :type "Float (double-precision)") (InputAction :type "InputAction Object Reference" :default "/Game/MyStuff/Input/IA_Move.IA_Move"))
  (bind (_returnvalue_roll _returnvalue_pitch _returnvalue_yaw) (`KismetMathLibrary.BreakRotator` (`self.GetControlRotation`)))
  (bind (_returnvalue_roll_2 _returnvalue_pitch_2 _returnvalue_yaw_2) (`KismetMathLibrary.BreakRotator` (`self.GetControlRotation`)))
  ;[1 1 1] Player Move
  (:`Triggered`
    (if (`self.CanMove`)
      ;;[1 1 1] Character Move Forward/Backward
      (`self.AddMovementInput` (`KismetMathLibrary.GetForwardVector` (`KismetMathLibrary.MakeRotator` 0.0 0.0 _returnvalue_yaw_2)) ActionValue_X)
      ;;[1 1 1] Character Move side to side
      (`self.AddMovementInput` (`KismetMathLibrary.GetRightVector` (`KismetMathLibrary.MakeRotator` 0.0 0.0 _returnvalue_yaw)) ActionValue_Y))))

(event `EnhancedInput|/Game/MyStuff/Input/IA_Look`
  (params (ActionValue :type "Vector2D Structure") (ElapsedSeconds :type "Float (double-precision)") (TriggeredSeconds :type "Float (double-precision)") (InputAction :type "InputAction Object Reference" :default "/Game/MyStuff/Input/IA_Look.IA_Look"))
  ;[1 1 1] Look
  (:`Triggered`
    (if (`self.CanMove`)
      (`self.AddControllerYawInput` (* ActionValue_X (`self.LookSensibility`)))
      (bind _result (`/Engine/EditorBlueprintResources/StandardMacros.NegateFloat` (* ActionValue_Y (`self.LookSensibility`)))
        (:`  `
          (`self.AddControllerPitchInput` _result))))))

(event `EnhancedInput|/Game/MyStuff/Input/IA_Crouch`
  (params (ActionValue :type Boolean) (ElapsedSeconds :type "Float (double-precision)") (TriggeredSeconds :type "Float (double-precision)") (InputAction :type "InputAction Object Reference" :default "/Game/MyStuff/Input/IA_Crouch.IA_Crouch"))
  ;[1 1 1] crouch
)

(event `EnhancedInput|/Game/MyStuff/Input/IA_Interact`
  (params (ActionValue :type Boolean) (ElapsedSeconds :type "Float (double-precision)") (TriggeredSeconds :type "Float (double-precision)") (InputAction :type "InputAction Object Reference" :default "/Game/MyStuff/Input/IA_Interact.IA_Interact"))
  ;[1 1 1] Interact
  (:`Started`
    (if (`self.CanMove`)
      (bind (_caninteract _currentinteractable _component) (`/Game/MyStuff/Blueprints/Components/BP_CheckForInteractables.CanInteract` (`self.CheckForInteractables`)))
      (if _caninteract
        (message `/Game/MyStuff/Blueprints/Interfaces/BPI_Puzzle.Interact` _currentinteractable self)
        (if (`KismetSystemLibrary.DoesImplementInterface` _currentinteractable "/Game/MyStuff/Blueprints/Interfaces/BPI_Rotator.BPI_Rotator_C")
          (message `/Game/MyStuff/Blueprints/Interfaces/BPI_Rotator.Rotator Call Up` _currentinteractable _component))))))

(event `EnhancedInput|/Game/MyStuff/Input/IA_Run`
  (params (ActionValue :type Boolean) (ElapsedSeconds :type "Float (double-precision)") (TriggeredSeconds :type "Float (double-precision)") (InputAction :type "InputAction Object Reference" :default "/Game/MyStuff/Input/IA_Run.IA_Run"))
  (bind _charactermovement (`self.CharacterMovement`))
  (:`Started`
    (set `CharacterMovementComponent.MaxWalkSpeed` (`self.Sprintsped`) _charactermovement)
    (set `self.headWobbleAmount` 10.0)
    (set `self.HeadWobbleSpeed` 40.0))
  (:`Completed`
    (set `CharacterMovementComponent.MaxWalkSpeed` (`self.Max Walk Speed`) _charactermovement)
    (set `self.headWobbleAmount` 6.0)
    (set `self.HeadWobbleSpeed` 0.5)))

(event `EnhancedInput|/Game/MyStuff/Input/IA_Flashlight`
  (params (ActionValue :type Boolean) (ElapsedSeconds :type "Float (double-precision)") (TriggeredSeconds :type "Float (double-precision)") (InputAction :type "InputAction Object Reference" :default "/Game/MyStuff/Input/IA_Flashlight.IA_Flashlight"))
  (bind _spotlight (`self.SpotLight`))
  (bind _spotlight1 (`self.SpotLight1`))
  ;[1 1 1] Falshlight
  (:`Started`
    (if (`self.CanMove`)
      (`SceneComponent.SetVisibility` _spotlight (not (`SceneComponent.bVisible` _spotlight)) false)
      (`SceneComponent.SetVisibility` _spotlight1 (not (`SceneComponent.bVisible` _spotlight1)) false))))

(event `EnhancedInput|/Game/MyStuff/Input/IA_DropObject`
  (params (ActionValue :type Boolean) (ElapsedSeconds :type "Float (double-precision)") (TriggeredSeconds :type "Float (double-precision)") (InputAction :type "InputAction Object Reference" :default "/Game/MyStuff/Input/IA_DropObject.IA_DropObject"))
  (:`Started`
    (`self.Drop Object`)))

(event `EnhancedInput|/Game/MyStuff/Input/IA_InspectObject`
  (params (ActionValue :type Boolean) (ElapsedSeconds :type "Float (double-precision)") (TriggeredSeconds :type "Float (double-precision)") (InputAction :type "InputAction Object Reference" :default "/Game/MyStuff/Input/IA_InspectObject.IA_InspectObject"))
  (bind _handslot (`self.HandSlot`))
  (:`Started`
    (`/Engine/EditorBlueprintResources/StandardMacros.IsValid` _handslot
      (:`Is Valid`
        (`/Game/MyStuff/Blueprints/BP_Pickup.Start Inspect` _handslot)))))

(event `EnhancedInput|/Game/MyStuff/Input/IA_Pause`
  (params (ActionValue :type Boolean) (ElapsedSeconds :type "Float (double-precision)") (TriggeredSeconds :type "Float (double-precision)") (InputAction :type "InputAction Object Reference" :default "/Game/MyStuff/Input/IA_Pause.IA_Pause"))
  ;[1 1 1] Pause game
  (:`Started`
    (`/Game/MyStuff/Blueprints/BP_Gamemode_Base.PauseGame` (`self.GameMode`))))

(fn `Add Mapping Context`
  (params (Remove :type Boolean))
  (bind _returnvalue (pcsubsystem `EnhancedInputLocalPlayerSubsystem` (`GameplayStatics.GetPlayerController` 0)))
  (bind _returnvalue_2 (pcsubsystem `EnhancedInputLocalPlayerSubsystem` (`GameplayStatics.GetPlayerController` 0)))
  (if Remove
    ;[0.4566 0 0] remove mapping Context
    (`/Engine/EditorBlueprintResources/StandardMacros.IsValid` _returnvalue
      (:`Is Valid`
        (`EnhancedInputSubsystemInterface.RemoveMappingContext` _returnvalue "/Game/MyStuff/Input/IMC_Player.IMC_Player" (struct)))
      (:`Is Not Valid`
        (`KismetSystemLibrary.PrintString` "BP_Player: Input system not found \nOops")))
    (else
      ;[0.2601 1 0.2388] Add mapping Context
      (`/Engine/EditorBlueprintResources/StandardMacros.IsValid` _returnvalue_2
        (:`Is Valid`
          (`EnhancedInputSubsystemInterface.AddMappingContext` _returnvalue_2 "/Game/MyStuff/Input/IMC_Player.IMC_Player" 0 (struct)))
        (:`Is Not Valid`
          (`KismetSystemLibrary.PrintString` "BP_Player: Input system not found \nOops"))))))

(fn `SetUpCamera`
  (bind _returnvalue (`GameplayStatics.GetPlayerCameraManager` 0))
  (set `PlayerCameraManager.ViewPitchMin` -80.0 _returnvalue)
  (set `PlayerCameraManager.ViewPitchMax` 89.0 _returnvalue))

(fn `UserConstructionScript`
  (bind _returnvalue (`AddComponent|NODE_AddBP_CheckForInteractables-0` :`Camera` (`self.Camera`)))
  (set `self.CheckForInteractables` _returnvalue))