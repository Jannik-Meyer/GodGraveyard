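; BP_GodTalks is an interactable actor that voices a god's line of dialogue.
; Highlighting applies an outline overlay to its cube, and interacting shows the Dialogue text in a WBP_God widget with a monster call sound.
; A second interaction, or losing highlight while talking, closes the widget.
; Closing then plays a level sequence if End is set, otherwise opens the "Remember" speech once through BP_Gamemode_Base.
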(event `self.SetHighlight`
  (params (On :type Boolean))
  (bind _cube (`self.Cube`))
  (if On
    (`MeshComponent.SetOverlayMaterial` _cube "/Game/MyStuff/Materials/Postprocess/NewFolder/M_Outline.M_Outline")
    (else
      (`MeshComponent.SetOverlayMaterial` _cube null)
      (if (`self.Talking?`)
        (`Widget.RemoveFromParent` (`self.UI`))
        (set `self.TalkIndex` -1)
        (set `self.UI` null)
        (set `self.Talking?` false)
        (if (`self.End`)
          (`MovieSceneSequencePlayer.Play` (`LevelSequenceActor.SequencePlayer` (`self.Sequence`)))
          (else
            (`/Engine/EditorBlueprintResources/StandardMacros.DoOnce` false
              (:`Completed`
                (bind _asbp_gamemode_base (cast `/Game/MyStuff/Blueprints/BP_Gamemode_Base` (`GameplayStatics.GetGameMode`)))
                (`/Game/MyStuff/Blueprints/BP_Gamemode_Base.OpenSpeech` _asbp_gamemode_base "Remember")))))))))

(event `self.Interact`
  (params (lastPossessed :type "Pawn Object Reference"))
  (bind _talkindex (`self.TalkIndex`))
  (set `self.Talking?` true)
  (`/Engine/EditorBlueprintResources/StandardMacros.IncrementInt` _talkindex
    (:`  `
      (if (< _talkindex 1)
        (`self.UI`
          (:`then`
            _)
          (:`else`
            (bind _returnvalue (`|CreateWidget` "/Game/MyStuff/UI/WBP_God.WBP_God_C" (`GameplayStatics.GetPlayerController` 0)))
            (bind _output_get (set `self.UI` _returnvalue))
            (`UserWidget.AddToViewport` _output_get 0)))
        (`TextBlock.SetText` (`/Game/MyStuff/UI/WBP_God.TalkText` (`self.UI`)) (`KismetTextLibrary.Conv_StringToText` (`self.Dialogue`)))
        (`GameplayStatics.PlaySoundAtLocation` "/Game/MyStuff/Sounds/god/creature-abstract-huge-monster-call-communicate-01.creature-abstract-huge-monster-call-communicate-01" (`SceneComponent.RelativeLocation` (`self.Cube`)) (struct) 1.0 1.0 0.0 null null null null)
        (else
          (`Widget.RemoveFromParent` (`self.UI`))
          (set `self.TalkIndex` -1)
          (set `self.UI` null)
          (set `self.Talking?` false)
          (if (`self.End`)
            (`MovieSceneSequencePlayer.Play` (`LevelSequenceActor.SequencePlayer` (`self.Sequence`)))
            (else
              (`/Engine/EditorBlueprintResources/StandardMacros.DoOnce` false
                (:`Completed`
                  (bind _asbp_gamemode_base (cast `/Game/MyStuff/Blueprints/BP_Gamemode_Base` (`GameplayStatics.GetGameMode`)))
                  (`/Game/MyStuff/Blueprints/BP_Gamemode_Base.OpenSpeech` _asbp_gamemode_base "Remember"))))))))))

(fn `Interactable`
  (returns (Interactable :type Boolean))
  (return true))

(fn `UserConstructionScript`)