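; BP_CorrectAnswer is a trigger actor that reports correct and wrong answers based on which tagged actor occupies it.
; An overlapping actor with the matching Tag calls CorrectMessage with +1 on the Target, and one leaving the collision component calls WrongMessage with -1.
; Both paths also fire an empty debug print, and the ClosertoEnd function is an empty stub.
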(event `self.ReceiveActorBeginOverlap`
  (params (OtherActor :type "Actor Object Reference"))
  (if (`self.ActorHasTag` OtherActor (`self.Tag`))
    (message `/Game/MyStuff/Blueprints/Interfaces/BPI_RiddleTrue.Correct` (`self.Target`) 1)
    (`KismetSystemLibrary.PrintString` "")))

(event `self.CollisionComponent.OnComponentEndOverlap`
  (params (OverlappedComponent :type "PrimitiveComponent Object Reference") (OtherActor :type "Actor Object Reference") (OtherComp :type "PrimitiveComponent Object Reference") (OtherBodyIndex :type Integer))
  (if (`self.ActorHasTag` OtherActor (`self.Tag`))
    (message `/Game/MyStuff/Blueprints/Interfaces/BPI_RiddleTrue.Wrong` (`self.Target`) -1)
    (`KismetSystemLibrary.PrintString` "")))

(fn `ClosertoEnd`
  (params (RightSacrifce :type Integer :default 0)))

(fn `UserConstructionScript`)