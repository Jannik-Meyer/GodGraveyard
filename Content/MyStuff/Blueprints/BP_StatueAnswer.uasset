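; Statue puzzle controller that tallies correct and false statue placements and tracks how many sacrifice rounds have been solved.
; CorrectStatue and FalsePosition adjust a running count, clamped at zero on the false path, and compare it to the required total on the correct path.
; Each match resets the count, messages its targets with the new stage and plays a sound.
; The third triggers a one-time ending message, then delayed GameMode statue speech and a monster call.
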(event `self.ReceiveBeginPlay`
  (set `self.Number` 0)
  (set `self.FullTruth` 0))

(event `/Game/MyStuff/Blueprints/Interfaces/BPI_StatueTrue.correctStatue`
  (params (yes :type Integer))
  (bind _fulltruth (`self.FullTruth`))
  (set `self.Number` (+ (`self.Number`) yes))
  (if (== (`self.Number`) (`self.Right Sacrifce`))
    (`KismetSystemLibrary.PrintText` "")
    (bind _result (`/Engine/EditorBlueprintResources/StandardMacros.IncrementInt` (`self.FullTruth`))
      (:`  `
        (`KismetSystemLibrary.PrintString` (`KismetStringLibrary.Conv_IntToString` _result))
        (set `self.Number` 0)
        (message `/Game/MyStuff/Blueprints/Interfaces/BPI_ChangeCode.ChangeCode` (`self.targets`) _fulltruth)
        (`FMODBlueprintStatics.PlayEvent2D` "/Game/FMOD/Events/Gods/creature-ghost-voice-abstract-short-02.creature-ghost-voice-abstract-short-02")
        (if (== 3 _fulltruth)
          (`/Engine/EditorBlueprintResources/StandardMacros.DoOnce` false
            (:`Completed`
              (message `/Game/MyStuff/Blueprints/Interfaces/BPI_UltimateTracker.TheEnddrawsnear` (`self.Target`) 0)
              (`KismetSystemLibrary.Delay` 2.0)
              (bind _asbp_gamemode_base (cast `/Game/MyStuff/Blueprints/BP_Gamemode_Base` (`GameplayStatics.GetGameMode`)))
              (`/Game/MyStuff/Blueprints/BP_Gamemode_Base.OpenSpeech` _asbp_gamemode_base "statue")
              (`FMODBlueprintStatics.PlayEvent2D` "/Game/FMOD/Events/Gods/creature-abstract-huge-monster-call-communicate-01.creature-abstract-huge-monster-call-communicate-01"))))))))

(event `/Game/MyStuff/Blueprints/Interfaces/BPI_StatueTrue.FalsePosition`
  (params (False :type Integer))
  (set `self.Number` (+ (`self.Number`) False))
  (if (< (`self.Number`) 0)
    (set `self.Number` 0)))

(fn `UserConstructionScript`)